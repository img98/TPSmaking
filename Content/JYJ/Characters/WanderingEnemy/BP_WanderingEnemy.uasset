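; BP_WanderingEnemy is a wandering enemy Blueprint that exposes AI blackboard state through getter functions.
; Two getters check that the AIController is valid, then read the InAttackRange bool and the AIState enum, converted to EAIState, from its blackboard.
; Tick and the construction script only call the parent, BeginPlay and overlap events are disabled placeholders, and NewFunction_0 is empty.
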(event `self.ReceiveTick`
  (params (DeltaSeconds :type "Float (single-precision)"))
  (`parent.ReceiveTick` DeltaSeconds))

(fn `GetBB_AIState`
  (returns (BB_AIState :type "EAIState Enum"))
  (bind _aicontroller (`self.AIController`)
    (:`then`
      (return (cast `EAIState` (`BlackboardComponent.GetValueAsEnum` (`AIBlueprintHelperLibrary.GetBlackboard` _aicontroller) "AIState"))))
    (:`else`)))

(fn `GetBB_InAttackRange`
  (returns (BB_InAttackRange :type Boolean))
  (bind _aicontroller (`self.AIController`)
    (:`then`
      (return (`BlackboardComponent.GetValueAsBool` (`AIBlueprintHelperLibrary.GetBlackboard` _aicontroller) "InAttackRange")))
    (:`else`)))

(fn `NewFunction_0`)

(fn `UserConstructionScript`
  (`parent.UserConstructionScript`))